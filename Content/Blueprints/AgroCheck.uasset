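; Behavior Tree node that handles enemy aggro detection, picking a target for the AI to follow.
; Each tick it sphere-traces DetectDistance around the controlled pawn, ignoring all EnemyAI actors, with debug drawing on.
; A Camera-channel line trace checks sight to each hit, writing TargetToFollow and TargetLocation if clear, otherwise clearing TargetToFollow.
; The last hit processed wins, and an empty sweep leaves the blackboard unchanged.
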(event `self.ReceiveTick`
  (params (OwnerActor :type "Actor Object Reference") (DeltaSeconds :type "Float (single-precision)"))
  (bind _returnvalue (`Actor.K2_GetActorLocation` (`Controller.K2_GetPawn` (`self.AI CON Ref`))))
  ;[1 1 1] Is AI_Con_Ref set?
  (if (not (!= (`self.AI CON Ref`) null))
    (bind _asenemy_ai_controller (cast `/Game/Blueprints/EnemyAiController` OwnerActor))
    (set `self.AI CON Ref` _asenemy_ai_controller))
  (bind _outactors (`GameplayStatics.GetAllActorsOfClass` "/Game/Blueprints/EnemyAI.EnemyAI_C"))
  (set `self.My Location` _returnvalue)
  (bind _outhits (`KismetSystemLibrary.SphereTraceMultiForObjects` _returnvalue (+ _returnvalue (0.0 0.0 15.0)) (`self.Detect Distance`) (`self.Desired Object Types`) false _outactors "ForDuration" true (struct :`R` 1.0 :`A` 1.0) (struct :`G` 1.0 :`A` 1.0) 1.0))
  (for _array_element _outhits
    (bind (_bblockinghit _binitialoverlap _time _location _impactpoint _normal _impactnormal _physmat _hitactor) (`GameplayStatics.BreakHitResult` _array_element))
    (bind _outhit (`KismetSystemLibrary.LineTraceSingle` (`self.My Location`) (`Actor.K2_GetActorLocation` _hitactor) "TraceTypeQuery2" false _outactors "ForDuration" true (struct :`R` 1.0 :`A` 1.0) (struct :`G` 1.0 :`A` 1.0) 2.0))
    (bind (_bblockinghit_2 _binitialoverlap_2 _time_2 _location_2 _impactpoint_2 _normal_2 _impactnormal_2 _physmat_2 _hitactor_2) (`GameplayStatics.BreakHitResult` _outhit))
    (if (== _hitactor_2 _hitactor)
      (`BTFunctionLibrary.SetBlackboardValueAsObject` (`self.Target to Follow`) _hitactor_2)
      (`BTFunctionLibrary.SetBlackboardValueAsVector` (`self.Target Location`) (`Actor.K2_GetActorLocation` _hitactor_2))
      (else
        (`BTFunctionLibrary.SetBlackboardValueAsObject` (`self.Target to Follow`))))))