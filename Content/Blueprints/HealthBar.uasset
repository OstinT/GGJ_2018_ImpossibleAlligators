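; HealthBar is an early-stage Blueprint that tracks player health as an array of components tagged "Health".
; BeginPlay enables input from the first player controller and fills the HealthNumber array from those components.
; The Dash input toggles IfDamaged through a FlipFlop.
; Tick prints the array length as a debug readout and checks IfDamaged, but that branch does nothing yet.
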(event `self.ReceiveBeginPlay`
  ;[1 1 1] Creates an array for the ammount of health the player has
  (`self.EnableInput` (`GameplayStatics.GetPlayerController` 0))
  (for _array_element (`self.GetComponentsByTag` "/Script/Engine.ActorComponent" "Health")
    (`KismetArrayLibrary.Array_Add` (`self.healthNumber`) _array_element)))

(event `InputAction|Dash`
  (params (Key :type "Key Structure"))
  (:`Pressed`
    (`/Engine/EditorBlueprintResources/StandardMacros.FlipFlop`
      (:`A`
        (set `self.ifDamaged` true))
      (:`B`
        (set `self.ifDamaged` false)))))

(event `self.ReceiveTick`
  (params (DeltaSeconds :type "Float (single-precision)"))
  (`KismetSystemLibrary.PrintString` (`KismetStringLibrary.Conv_IntToString` (`KismetArrayLibrary.Array_Length` (`self.healthNumber`))) true true (struct :`R` 0.989583 :`G` 0.979167 :`B` 1.0 :`A` 1.0))
  (if (`self.ifDamaged`)
    _))

(fn `UserConstructionScript`)