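; Enemy actor Blueprint with a small health pool and a temporary words display.
; BeginPlay initializes Health; TakeDamage decrements it by one and destroys the actor when it runs out.
; DisplayWords shows the EnemyWords component briefly, then hides it again after a delay.
; Tick prints the current Health every frame as debug output.
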(event `self.ReceiveBeginPlay`
  (set `self.Health` 3))

(event `DisplayWords`
  (`SceneComponent.SetHiddenInGame` (`self.EnemyWords`) false false)
  (`KismetSystemLibrary.Delay` 1.0)
  (`SceneComponent.SetHiddenInGame` (`self.EnemyWords`) true false))

(event `self.ReceiveTick`
  (params (DeltaSeconds :type "Float (single-precision)"))
  (`KismetSystemLibrary.PrintString` (`KismetStringLibrary.Conv_IntToString` (`self.Health`))))

(fn `Take Damage`
  (`/Engine/EditorBlueprintResources/StandardMacros.DecrementInt` (`self.Health`)
    (:`  `
      (if (<= (`self.Health`) 0)
        (`self.K2_DestroyActor`)))))

(fn `UserConstructionScript`)